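; BP_Weapon is a weapon pickup actor that the third-person character collects with the Weapon Pickup input.
; Its PlayerDetect overlap stores an unarmed character as PlayerRef and shows the interact UI, then clears both when that character leaves.
; Pressing the input while PlayerRef is valid and unarmed sets HasWeapon, enables the gun on the HotBar and destroys the pickup.
; The UI clear after pickup reuses the end-overlap cast result rather than PlayerRef.
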(event `InputAction|Weapon Pickup` :consume false
  (params (Key :type "Key Structure"))
  (bind _playerref (`self.PlayerRef`))
  (:`Pressed`
    (`/Engine/EditorBlueprintResources/StandardMacros.IsValid` _playerref
      (:`Is Valid`
        (if (not (`/Game/ThirdPerson/Blueprints/BP_ThirdPersonCharacter.HasWeapon` _playerref))
          (set `/Game/ThirdPerson/Blueprints/BP_ThirdPersonCharacter.HasWeapon` true _playerref)
          (`/Game/Paul/WBP_Hotbar.EnableGun` (`/Game/ThirdPerson/Blueprints/BP_ThirdPersonCharacter.HotBar` _playerref))
          (`self.K2_DestroyActor` self)
          (`/Game/ThirdPerson/Blueprints/BP_ThirdPersonCharacter.ClearInteractUI` (stale `self.PlayerDetect.OnComponentEndOverlap` _asbp_third_person_character) :!label _label))))))

(event `self.PlayerDetect.OnComponentBeginOverlap`
  (params (OverlappedComponent :type "PrimitiveComponent Object Reference") (OtherActor :type "Actor Object Reference") (OtherComp :type "PrimitiveComponent Object Reference") (OtherBodyIndex :type Integer) (bFromSweep :type Boolean) (SweepResult :type "HitResult Structure (by ref)"))
  (bind _asbp_third_person_character (cast `/Game/ThirdPerson/Blueprints/BP_ThirdPersonCharacter` OtherActor))
  (if (not (`/Game/ThirdPerson/Blueprints/BP_ThirdPersonCharacter.HasWeapon` _asbp_third_person_character))
    (bind _output_get (set `self.PlayerRef` _asbp_third_person_character))
    (`/Game/ThirdPerson/Blueprints/BP_ThirdPersonCharacter.InteractUI` _output_get)))

(event `self.PlayerDetect.OnComponentEndOverlap`
  (params (OverlappedComponent :type "PrimitiveComponent Object Reference") (OtherActor :type "Actor Object Reference") (OtherComp :type "PrimitiveComponent Object Reference") (OtherBodyIndex :type Integer))
  (bind _asbp_third_person_character (cast `/Game/ThirdPerson/Blueprints/BP_ThirdPersonCharacter` OtherActor))
  (if (not (`/Game/ThirdPerson/Blueprints/BP_ThirdPersonCharacter.HasWeapon` _asbp_third_person_character))
    (set `self.PlayerRef` null)
    (goto _label)))

(fn `UserConstructionScript`)